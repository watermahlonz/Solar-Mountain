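; Audio manager Blueprint that centralizes one-shot sound effects for player actions and level events such as jumping, dashing, checkpoints, doors, respawn and victory.
; Each event has its own function that plays an assigned sound variable as non-spatialized 2D audio.
; The jump function picks a random entry from an array of jump sounds for variation, while the others each play a single fixed sound.
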(fn PlayMySoundAbility
  (Audio|PlaySound2D 0 (LocalVariables|GetAbilitySound) 1.0 1.0 0.0 0 0))

(fn PlayMySoundCheckpoint
  (Audio|PlaySound2D 0 (LocalVariables|GetCheckpointSound) 1.0 1.0 0.0 0 0))

(fn PlayMySoundDash
  (Audio|PlaySound2D 0 (LocalVariables|GetDashSound) 1.0 1.0 0.0 0 0))

(fn PlayMySoundDoorActivate
  (Audio|PlaySound2D 0 (LocalVariables|GetDoorActivateSound) 1.0 1.0 0.0 0 0))

(fn PlayMySoundJump
  (Audio|PlaySound2D 0 (.OutItem (Utilities|Array|Random (LocalVariables|GetJumpSounds))) 1.0 1.0 0.0 0 0))

(fn PlayMySoundLanding
  (Audio|PlaySound2D 0 (LocalVariables|GetLandingSound) 1.0 1.0 0.0 0 0))

(fn PlayMySoundRespawn
  (Audio|PlaySound2D 0 (LocalVariables|GetRespawnSound) 1.0 1.0 0.0 0 0))

(fn PlayMySoundVictory
  (Audio|PlaySound2D 0 (LocalVariables|GetVictorySound) 1.0 1.0 0.0 0 0))