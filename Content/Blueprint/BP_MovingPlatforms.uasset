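; Moving platform that travels between its start and a configurable MoveToPos offset, set as InterpToMovement control points in the construction script.
; When BP_PlayerCharacter enters its Box, it enables movement in PingPong mode, plays a sound and switches the plane to a solar material.
; Leaving switches to OneShotReverse.
; Tick gates the movement component's ticking, and on zero velocity clears the player flag, restarts movement and restores the floor material.
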(event OnComponentBeginOverlap(Box)
  (params (OverlappedComponent :type Primitive%20Component%20Object%20Reference) (OtherActor :type Actor%20Object%20Reference) (OtherComp :type Primitive%20Component%20Object%20Reference) (OtherBodyIndex :type Integer) (bFromSweep :type Boolean) (SweepResult :type Hit%20Result%20Structure%20%28by%20ref%29))
  (Utilities|Casting|CastToBP_PlayerCharacter OtherActor)
  (Variables|Default|SetIs%20Player%20Colliding true)
  (Audio|PlaySound2D "/Game/Assets/Audio/388306__the_yura__flying-plane.388306__the_yura__flying-plane" 1.0 1.0 0.0 0 0)
  (Variables|/Script/Engine.InterpToMovementComponent|SetBehaviourType (Variables|Default|GetInterpToMovement) "PingPong")
  (Rendering|Material|SetMaterial (Variables|Default|GetPlane) 0 "/Game/Assets/Materials/M_Solar.M_Solar"))

(event OnComponentEndOverlap(Box)
  (params (OverlappedComponent :type Primitive%20Component%20Object%20Reference) (OtherActor :type Actor%20Object%20Reference) (OtherComp :type Primitive%20Component%20Object%20Reference) (OtherBodyIndex :type Integer))
  (Utilities|Casting|CastToBP_PlayerCharacter OtherActor)
  (Variables|/Script/Engine.InterpToMovementComponent|SetBehaviourType (Variables|Default|GetInterpToMovement) "OneShot_Reverse"))

(event EventBeginPlay)

(event EventTick
  (params (DeltaSeconds :type Float%20%28single-precision%29))
  (bind _interptomovement (Variables|Default|GetInterpToMovement))
  (if (Variables|Default|GetIs%20Player%20Colliding)
    (Components|Tick|SetComponentTickEnabled _interptomovement true)
    (if (Utilities|Operators|EqualEqual :A (Transformation|GetVelocity))
      (Variables|Default|SetIs%20Player%20Colliding false)
      (Class|InterptoMovementComponent|RestartMovement (Variables|Default|GetInterpToMovement) 1.0)
      (Rendering|Material|SetMaterial (Variables|Default|GetPlane) 0 "/Game/StarterContent/Materials/M_Basic_Floor.M_Basic_Floor"))
    (else
      (Components|Tick|SetComponentTickEnabled _interptomovement false))))

(fn ConstructionScript
  (bind _interptomovement (Variables|Default|GetInterpToMovement))
  (Class|InterptoMovementComponent|AddControlPointPosition _interptomovement "0, 0, 0" true)
  (Class|InterptoMovementComponent|AddControlPointPosition _interptomovement (Variables|Default|GetMoveToPos) true))